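; Game manager that triggers item spawns through references to wooden plank, firewood and fruit spawners.
; On BeginPlay, it spawns a plank and firewood slightly above their respective spawners.
; SpawnItemsByTree takes a tree location and spawns fruit and firewood at fixed offsets around and below it.
; Item creation is delegated to each spawner's SpawnItem call, so the manager only chooses when and where.
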(event Custom|SpawnItemsByTree
  (params (Tree%20Location :type Vector))
  (Default|SpawnItem (Variables|Default|GetFruit%20Spawner%20Ref) (+ Tree%20Location "200.000000,100.000000,-200.000000"))
  (Default|SpawnItem (Variables|Default|GetFirewood%20Spawner%20Ref) (+ Tree%20Location "-150.000000,-200.000000,-200.000000")))

(event EventBeginPlay
  (bind _wooden_plank_spawner_ref (Variables|Default|GetWooden%20Plank%20Spawner%20Ref))
  (bind _firewood_spawner_ref (Variables|Default|GetFirewood%20Spawner%20Ref))
  (Default|SpawnItem _wooden_plank_spawner_ref (+ (Transformation|GetActorLocation _wooden_plank_spawner_ref) "0.000000,0.000000,60.000000"))
  (Default|SpawnItem _firewood_spawner_ref (+ (Transformation|GetActorLocation _firewood_spawner_ref) "0.000000,0.000000,60.000000")))

(fn ConstructionScript)