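; BP_NavEnemy is an enemy pawn that patrols waypoints, chases the player and deals contact damage.
; A two-state switch drives AI MoveTo, with Tick advancing patrol along a looping waypoint list, wrapped at a hardcoded index.
; PawnSensing sightings trigger a chase, and a retriggerable delay resumes patrol once sightings stop.
; Box overlap damages BP_Player with a short cooldown, and ending that overlap restarts the chase.
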(event OnComponentBeginOverlap(Box)
  (params (OverlappedComponent :type Primitive%20Component%20Object%20Reference) (OtherActor :type Actor%20Object%20Reference) (OtherComp :type Primitive%20Component%20Object%20Reference) (OtherBodyIndex :type Integer) (bFromSweep :type Boolean) (SweepResult :type Hit%20Result%20Structure%20%28by%20ref%29))
  (if (Actor|ActorHasTag OtherActor "Player")
    (if (Variables|Default|GetCan%20Attack)
      (bind _asbp_player (Utilities|Casting|CastToBP_Player OtherActor))
      (Default|TakeDamage _asbp_player)
      (Variables|Default|SetCan%20Attack false)
      (Utilities|FlowControl|Delay 0.5)
      (Variables|Default|SetCan%20Attack true))))

(event OnComponentEndOverlap(Box)
  (params (OverlappedComponent :type Primitive%20Component%20Object%20Reference) (OtherActor :type Actor%20Object%20Reference) (OtherComp :type Primitive%20Component%20Object%20Reference) (OtherBodyIndex :type Integer))
  (if (Actor|ActorHasTag OtherActor "Player")
    (CallFunction|Chase)))

(event OnSeePawn(PawnSensing)
  (params (Pawn :type Pawn%20Object%20Reference))
  (Utilities|FlowControl|Sequence
    (:then_0
      (CallFunction|Chase))
    (:then_1
      (Utilities|FlowControl|RetriggerableDelay 1.5)
      (CallFunction|MovetoNextWaypoint))))

(event Custom|Chase
  (CallFunction|SwitchState "NewEnumerator1")
  (CallFunction|LocatePlayer)
  (AI|AIMoveTo self "0, 0, 0" (Variables|Default|GetPlayer) 5.0 false))

(event Custom|StartPatrolling
  (CallFunction|SwitchState "NewEnumerator0")
  (bind _output_get (Variables|Default|SetDestination (Transformation|GetActorLocation (Utilities|Array|Get(acopy) (Variables|Default|GetWaypoints)))))
  (AI|AIMoveTo self _output_get 0 5.0 false))

(event Custom|MoveToNextWaypoint
  (CallFunction|SwitchState "NewEnumerator0")
  (bind _output (CallFunction|GetNextWaypoint))
  (bind _output_get (Variables|Default|SetDestination (Transformation|GetActorLocation _output)))
  (AI|AIMoveTo self _output_get 0 5.0 false))

(event EventBeginPlay
  (CallFunction|StartPatrolling))

(event EventTick
  (params (DeltaSeconds :type Float%20%28single-precision%29))
  (switch Utilities|FlowControl|Switch|SwitchonENavEnemyState (Variables|Default|GetCurrent%20State)
    (:NewEnumerator0
      (if (<= (Math|Vector|Distance(Vector) (Variables|Default|GetDestination) (Transformation|GetActorLocation)) 5e+01)
        (CallFunction|MovetoNextWaypoint)))))

(fn ConstructionScript)

(fn LocatePlayer
  (bind _outactors (Actor|GetAllActorsOfClass "/Game/Blueprints/Player/BP_Player.BP_Player_C"))
  (Variables|Default|SetPlayer (Utilities|Array|Get(acopy) _outactors)))

(fn GetNextWaypoint
  (if (>= (Variables|Default|GetWaypoint%20Index) 5)
    (Variables|Default|SetWaypoint%20Index 0)
    (else
      (Variables|Default|SetWaypoint%20Index (+ (Variables|Default|GetWaypoint%20Index) 1))))
  (return (Utilities|Array|Get(acopy) (Variables|Default|GetWaypoints) (Variables|Default|GetWaypoint%20Index))))

(fn SwitchState
  (params (NewState :type ENavEnemyState%20Enum :default "NewEnumerator0"))
  (Variables|Default|SetCurrent%20State NewState)
  (switch Utilities|FlowControl|Switch|SwitchonENavEnemyState NewState
    (:NewEnumerator0
      (Development|PrintString "Patrolling"))
    (:NewEnumerator1
      (Development|PrintString "Chasing"))))