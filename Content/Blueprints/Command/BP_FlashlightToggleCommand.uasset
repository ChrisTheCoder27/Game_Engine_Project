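; Command object that toggles the player's flashlight, with Execute and Undo events following the command pattern.
; Execute casts the target actor to BP_Player, sets its SpotLight to the new intensity and marks FlashlightOn true.
; Undo restores the previous intensity and clears the flag, so each command represents switching the light on and reverting it.
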(event EventUndo
  (bind _targetactor (Variables|Default|GetTargetActor))
  (Utilities|IsValid _targetactor
    (:Is%20Valid
      (bind _asbp_player (Utilities|Casting|CastToBP_Player _targetactor))
      (Rendering|Components|Light|SetIntensity (Variables|/Game/Blueprints/Player/BP_Player.BP_Player_C|GetSpotLight _asbp_player) (Variables|Default|GetPreviousIntensity))
      (Variables|/Game/Blueprints/Player/BP_Player.BP_Player_C|SetFlashlightOn _asbp_player false))))

(event EventExecute
  (bind _targetactor (Variables|Default|GetTargetActor))
  (Utilities|IsValid _targetactor
    (:Is%20Valid
      (bind _asbp_player (Utilities|Casting|CastToBP_Player _targetactor))
      (Rendering|Components|Light|SetIntensity (Variables|/Game/Blueprints/Player/BP_Player.BP_Player_C|GetSpotLight _asbp_player) (Variables|Default|GetNewIntensity))
      (Variables|/Game/Blueprints/Player/BP_Player.BP_Player_C|SetFlashlightOn _asbp_player true))))

(fn ConstructionScript)