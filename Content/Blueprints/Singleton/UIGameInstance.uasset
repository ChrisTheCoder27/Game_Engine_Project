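; Game instance that holds the player's health, stamina and countdown timer and pushes each change to the PlayerHUD's UI widget.
; Health is capped at the top, and depleting it reloads the current level and resets health and timer.
; Stamina changes in single-point steps, and draining past zero notifies every BPI_Observer actor, an observer-style broadcast.
; The timer counts down by world delta time and stops updating at zero.
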(fn ChangeHealth
  (params (Amount :type Float%20%28double-precision%29))
  (Math|Float|CompareFloat (+ (Variables|Default|GetCurrentHealth) Amount) 0.0
    (:>
      (bind _output_get (Variables|Default|SetCurrentHealth (+ (Variables|Default|GetCurrentHealth) Amount)))
      (Math|Float|CompareFloat _output_get 1e+02
        (:>
          (Variables|Default|SetCurrentHealth 1e+02))
        (:==
          _)
        (:<
          _))
      (bind _asplayer_hud (Utilities|Casting|CastToPlayerHUD (HUD|GetHUD (Game|GetPlayerController 0))))
      (Default|UpdateHealthBar (Variables|/Game/Blueprints/Singleton/PlayerHUD.PlayerHUD_C|GetUI%20Reference _asplayer_hud) (Variables|Default|GetCurrentHealth)))
    (:==
      (bind _returnvalue (Game|GetCurrentLevelName true :!label _label))
      (Game|OpenLevel(byName) (Utilities|String|StringToName _returnvalue))
      (Variables|Default|SetCurrentHealth 1e+02)
      (Variables|Default|SetTimer 6e+01))
    (:<
      (goto _label))))

(fn DecreaseStamina
  (Math|Float|CompareFloat (- (Variables|Default|GetCurrentStamina) 1.0) 0.0
    (:>
      (Variables|Default|SetCurrentStamina (- (Variables|Default|GetCurrentStamina) 1.0) :!label _label)
      (bind _asplayer_hud (Utilities|Casting|CastToPlayerHUD (HUD|GetHUD (Game|GetPlayerController 0))))
      (Default|UpdateStaminaBar (Variables|/Game/Blueprints/Singleton/PlayerHUD.PlayerHUD_C|GetUI%20Reference _asplayer_hud) (Variables|Default|GetCurrentStamina)))
    (:==
      (goto _label))
    (:<
      (bind _outactors (Actor|GetAllActorswithInterface "/Game/Blueprints/Observer/BPI_Observer.BPI_Observer_C"))
      (for _array_element _outactors
        (Class|BPIObserver|Notify(Message) _array_element)))))

(fn IncreaseStamina
  (Math|Float|CompareFloat (+ (Variables|Default|GetCurrentStamina) 1.0) 1e+02
    (:==
      _)
    (:<
      _))
  (Variables|Default|SetCurrentStamina (+ (Variables|Default|GetCurrentStamina) 1.0))
  (bind _asplayer_hud (Utilities|Casting|CastToPlayerHUD (HUD|GetHUD (Game|GetPlayerController 0))))
  (Default|UpdateStaminaBar (Variables|/Game/Blueprints/Singleton/PlayerHUD.PlayerHUD_C|GetUI%20Reference _asplayer_hud) (Variables|Default|GetCurrentStamina)))

(fn UpdateTimer
  (Math|Float|CompareFloat (Math|Float|Clamp(Float) (- (Variables|Default|GetTimer) (Utilities|Time|GetWorldDeltaSeconds)) 0.0 (Variables|Default|GetTimer)) 0.0
    (:>
      (Variables|Default|SetTimer (Math|Float|Clamp(Float) (- (Variables|Default|GetTimer) (Utilities|Time|GetWorldDeltaSeconds)) 0.0 (Variables|Default|GetTimer)))
      (bind _asplayer_hud (Utilities|Casting|CastToPlayerHUD (HUD|GetHUD (Game|GetPlayerController 0))))
      (Default|UpdateTimerText (Variables|/Game/Blueprints/Singleton/PlayerHUD.PlayerHUD_C|GetUI%20Reference _asplayer_hud) (Variables|Default|GetTimer)))))